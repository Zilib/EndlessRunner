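; CorridorStraight is a straight corridor Blueprint that places a coin pickup when it begins play.
; On BeginPlay it picks one of three row sockets on CorridorMesh at random and spawns a Coin_BP at that socket's location.
; The overlap and tick events are disabled stubs, and the construction script is empty.
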(event EventBeginPlay
  (Game|SpawnActorfromClass "/Game/Blueprints/Coin_BP.Coin_BP_C" (Math|Conversions|ToTransform(Vector) (Transformation|GetSocketLocation (Variables|Default|GetCorridorMesh) (Utilities|Select :Index (Math|Random|RandomInteger 3) :Option%200 (Utilities|String|StringToName (Utilities|String|ToString(Text) (Utilities|Text|ToText(Name) "SecondRowSpawn1"))) :Option%201 (Utilities|String|StringToName (Utilities|String|ToString(Text) (Utilities|Text|ToText(Name) "ThirdRowSpawn1"))) :Option%202 (Utilities|String|StringToName (Utilities|String|ToString(Text) (Utilities|Text|ToText(Name) "FirstRowSpawn1")))))) "Undefined" 0 0))

(event Collision|EventActorBeginOverlap
  (params (OtherActor :type Actor%20Object%20Reference)))

(event EventTick
  (params (DeltaSeconds :type Float%20%28single-precision%29)))

(fn ConstructionScript)