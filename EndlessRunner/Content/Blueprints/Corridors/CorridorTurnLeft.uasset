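; CorridorTurnLeft is a corridor actor that turns the runner character left when it enters the collision box.
; The overlap checks the other actor's name against the runner name stored in MyGameInstance, then plays the TurnLeft timeline.
; Each update passes the change in TotalTurnValue to TurnARunner on player 0's character, applying the turn incrementally.
; IsActive is only ever set false here, so its guard never blocks retriggering.
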(event OnComponentBeginOverlap(CollisionBox)
  (params (OverlappedComponent :type Primitive%20Component%20Object%20Reference) (OtherActor :type Actor%20Object%20Reference) (OtherComp :type Primitive%20Component%20Object%20Reference) (OtherBodyIndex :type Integer) (bFromSweep :type Boolean) (SweepResult :type Hit%20Result%20Structure%20%28by%20ref%29))
  (if (not (Variables|Default|GetisActive))
    (bind _asmy_game_instance (Utilities|Casting|CastToMyGameInstance (Game|GetGameInstance)))
    (if (Utilities|Enum|Equal(Enum) (Variables|/Script/EndlessRunner.MyGameInstance|GetRunnerBPName _asmy_game_instance) (Utilities|GetObjectName OtherActor))
      (Variables|Default|SetTimelineDelta 0.0)
      (bind _asrunner_character_bp (Utilities|Casting|CastToRunnerCharacter_BP (Game|GetPlayerCharacter 0)))
      (bind _totalturnvalue (Timeline|Turn%20left Play)
        (:Update
          (Class|RunnerCharacter|TurnARunner _asrunner_character_bp (- _totalturnvalue (Variables|Default|GetTimelineDelta)))
          (Variables|Default|SetTimelineDelta _totalturnvalue)
          (Variables|Default|SetisActive false))))))

(event EventBeginPlay
  (Variables|Default|SetisActive false))

(fn ConstructionScript)