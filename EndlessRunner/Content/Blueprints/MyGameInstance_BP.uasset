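; Game instance that handles online version checking and scoreboard downloads through VaRest HTTP requests.
; On Init it queries a hardcoded server for the newest version and download URL, which IsTheNewestVersion compares against the running version.
; LoadFromDatabase clears the temporary array and posts to a PHP scoreboard API on the configured server.
; LoadDataToVariable decodes that JSON, reading name and score by field position, then rebuilds the ScoreBoard table.
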(event Custom|Cannot%20show%20variable
  (params (Request :type Va%20Rest%20Request%20JSON%20Object%20Reference))
  (Variables|Default|SetRequest%20Complet false))

(event Custom|Load%20Data%20To%20Variable
  (params (Request :type Va%20Rest%20Request%20JSON%20Object%20Reference))
  (bind _active_data_object (Variables|ScoreBoard|GetActive%20Data%20Object))
  (bind _scoreboard (Variables|ScoreBoard|GetScoreBoard))
  ;[1 1 1] Get records from database and save it to variable
  (bind _returnvalue (Class|VaRestRequestJSON|GetResponseContentasString Request false))
  (Class|VaRestJsonObject|DecodeJson _active_data_object _returnvalue false)
  (for _array_element (Class|VaRestJsonObject|GetFieldNames _active_data_object)
    (for (_array_element_2 _array_index) (Class|VaRestJsonObject|GetFieldNames (Class|VaRestJsonObject|GetObjectField (Variables|ScoreBoard|GetActive%20Data%20Object) _array_element))
      (switch int _array_index
        (:0
          (Class|MyGameInstance|SetPlayerName (Class|VaRestJsonObject|GetStringField (Class|VaRestJsonObject|GetObjectField (Variables|ScoreBoard|GetActive%20Data%20Object) _array_element) _array_element_2)))
        (:1
          (Class|MyGameInstance|SetScore (Math|Conversions|ToInteger(Byte) (Class|VaRestJsonObject|GetStringField (Class|VaRestJsonObject|GetObjectField (Variables|ScoreBoard|GetActive%20Data%20Object) _array_element) _array_element_2))))))
    (Class|MyGameInstance|AddtoData))
  (Utilities|FlowControl|Sequence
    (:then_0
      (Default|ClearTable _scoreboard))
    (:then_1
      (Default|LoadData _scoreboard))))

(event EventInit
  (CallFunction|GetNumberOftheNewestVersion))

(fn LoadfromDatabase
  ;[1 1 1] Every time, when it is called load new data
  (Class|MyGameInstance|ClearTemporaryArray)
  ;[1 1 1] Send request for to a database for a scoreboard table
  (bind _returnvalue (Class|VaRestRequestJSON|ConstructVaRestRequestExt "POST" "x_www_form_urlencoded_url"))
  (bind _output_get (Variables|ScoreBoard|SetActive%20Data%20Request _returnvalue))
  (bind _returnvalue_2 (Class|VaRestJsonObject|ConstructVaRestJsonObject))
  (bind _output_get_2 (Variables|ScoreBoard|SetActive%20Data%20Object _returnvalue_2))
  (Class|VaRestRequestJSON|SetRequestObject _output_get _output_get_2)
  (EventDispatchers|BindEventtoOnRequestComplete _output_get (EventDispatchers|CreateEvent :!event Custom|Load%20Data%20To%20Variable))
  (bind _returnvalue_3 (Class|MyGameInstance|GetServerIP))
  (Class|VaRestRequestJSON|ProcessURL _output_get (Utilities|String|Append _returnvalue_3 "/ScoreBoardApi/index2.php")))

(fn GetNumberOftheNewestVersion
  ;[1 1 1] Make request, and check which version is the newest
  (bind _returnvalue (Class|VaRestRequestJSON|ConstructVaRestRequestExt "GET" "x_www_form_urlencoded_url"))
  (bind _output_get (Variables|GameVersion|SetActive%20Version%20Request _returnvalue))
  (bind _returnvalue_2 (Class|VaRestJsonObject|ConstructVaRestJsonObject))
  (bind _output_get_2 (Variables|GameVersion|SetActive%20Version%20Object _returnvalue_2))
  (Class|VaRestRequestJSON|SetRequestObject _returnvalue _output_get_2)
  (EventDispatchers|BindEventtoOnRequestComplete _returnvalue (EventDispatchers|CreateEvent :!event SavetoVariablesNewestVersionGameInformation))
  (EventDispatchers|BindEventtoOnRequestFail _output_get (EventDispatchers|CreateEvent :!event Custom|Cannot%20show%20variable))
  (Class|VaRestRequestJSON|ProcessURL _returnvalue "http://139.59.133.82/"))

(fn SavetoVariablesNewestVersionGameInformation
  (params (Request :type Va%20Rest%20Request%20JSON%20Object%20Reference))
  (bind _returnvalue (Class|VaRestRequestJSON|GetRequestObject Request))
  (Variables|Default|SetRequest%20Complet true)
  (bind _returnvalue_2 (Class|VaRestRequestJSON|GetResponseContentasString Request false))
  (Class|VaRestJsonObject|DecodeJson _returnvalue _returnvalue_2 false)
  (Variables|GameVersion|SetDownloadURL (Class|VaRestJsonObject|GetStringField _returnvalue "DownloadURL"))
  (Variables|GameVersion|SetNewestGameVersion (Class|VaRestJsonObject|GetStringField _returnvalue "Version")))

(fn IstheNewestVersion
  (return (and (Variables|Default|GetRequest%20Complet) (Utilities|Enum|Equal(Enum) (Variables|GameVersion|GetNewestGameVersion) (Class|MyGameInstance|GetGameVersion)))))