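; MapSpawner_BP is a map spawner that extends a corridor over time, one segment after another.
; A Delay on Tick paces spawning to roughly once per second.
; A counter starting at one makes every fifth segment a corner and the rest straight.
; Meshes are looked up by name in the StaticMeshes map and passed to SpawnNextCorridor, which is defined outside these graphs.
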(event EventTick
  (params (DeltaSeconds :type Float%20%28single-precision%29))
  (bind _self self)
  (Utilities|FlowControl|Delay 1.0)
  (if (== (Math|Integer|%(Integer) (Variables|Default|GetCounterToChangeMesh) 5) 0)
    (Class|MapSpawner|SpawnNextCorridor _self (.Value (Utilities|Map|Find (Variables|Default|GetStaticMeshes) "Corner")))
    (else
      (Class|MapSpawner|SpawnNextCorridor _self (.Value (Utilities|Map|Find (Variables|Default|GetStaticMeshes) "Straight")))))
  (Math|Integer|IncrementInt (Variables|Default|GetCounterToChangeMesh)))

(event EventBeginPlay
  (Variables|Default|SetCounterToChangeMesh 1))

(fn ConstructionScript)